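; Demo actor that loads a Player Zero avatar through its PlayerZeroLoader component.
; On BeginPlay it calls LoadAvatar if the loader already has a non-empty avatar ID.
; LoadAvatar stores the given ID on the loader, starts the load with a high mesh LOD and texture atlas config, then prints the ID.
; The load-complete event is an empty stub.
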(event OnAvatarLoadComplete(PlayerZeroLoader)
  (params (LoadedMeshComponent :type Skeletal%20Mesh%20Component%20Object%20Reference)))

(event EventBeginPlay
  (bind _playerzeroloader (Variables|Default|GetPlayerZeroLoader))
  (bind _avatarid (Variables|/Script/PlayerZero.PlayerZeroLoaderComponent|GetAvatarId _playerzeroloader))
  ;[1 1 1] Try load avatar on start
  (if (not (Utilities|Array|IsEmpty _avatarid))
    (CallFunction|LoadAvatar _avatarid)))

(event Collision|EventActorBeginOverlap
  (params (OtherActor :type Actor%20Object%20Reference)))

(event EventTick
  (params (DeltaSeconds :type Float%20%28single-precision%29)))

(fn ConstructionScript)

(fn LoadAvatar
  (params (AvatarId :type String))
  (bind _playerzeroloader (Variables|Default|GetPlayerZeroLoader))
  (bind _output_get (Variables|/Script/PlayerZero.PlayerZeroLoaderComponent|SetAvatarId _playerzeroloader AvatarId))
  (Class|PlayerZeroLoaderComponent|LoadAvatar _playerzeroloader (Utilities|Struct|MakeCharacterConfig "High" "High" "High" "Limit_1024" "BaseColor" "Viseme_aa" "None"))
  (Development|PrintString (Utilities|String|Append "Load Avatar called with avatar ID:" _output_get)))